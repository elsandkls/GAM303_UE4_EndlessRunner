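; Endless-runner floor tile that spawns obstacles and keeps the track going as the player advances.
; On BeginPlay it randomly places at most one Obstacle on one of three lane arrows and stores its SpawnPoint location as NewSpawnPoint.
; When the character overlaps the Box, it has the game mode spawn another tile, adds multiplier-scaled points and raises walk speed within a clamp.
; The tile then destroys itself after a short delay.
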(event `self.ReceiveBeginPlay`
  (`self.SpawnObstacles`)
  (set `self.NewSpawnPoint` (`KismetMathLibrary.Conv_VectorToTransform` (`SceneComponent.K2_GetComponentLocation` (`self.SpawnPoint`)))))

(event `self.Box.OnComponentBeginOverlap`
  (params (OverlappedComponent :type "PrimitiveComponent Object Reference") (OtherActor :type "Actor Object Reference") (OtherComp :type "PrimitiveComponent Object Reference") (OtherBodyIndex :type Integer) (bFromSweep :type Boolean) (SweepResult :type "HitResult Structure (by ref)"))
  (set `self.NewSpawnPoint` (`KismetMathLibrary.Conv_VectorToTransform` (`SceneComponent.K2_GetComponentLocation` (`self.SpawnPoint`))))
  (cast `/Game/ThirdPersonBP/Blueprints/ThirdPersonCharacter` OtherActor)
  (bind _asthird_person_game_mode (cast `/Game/ThirdPersonBP/Blueprints/ThirdPersonGameMode` (`GameplayStatics.GetGameMode`)))
  (`/Game/ThirdPersonBP/Blueprints/ThirdPersonGameMode.SpawnTile` _asthird_person_game_mode)
  (bind _asthird_person_game_mode_2 (cast `/Game/ThirdPersonBP/Blueprints/ThirdPersonGameMode` (`GameplayStatics.GetGameMode`)))
  (set `/Game/ThirdPersonBP/Blueprints/ThirdPersonGameMode.CurrentPoints` (+ (`/Game/ThirdPersonBP/Blueprints/ThirdPersonGameMode.CurrentPoints` _asthird_person_game_mode_2) (* (`/Game/ThirdPersonBP/Blueprints/ThirdPersonGameMode.PointsMultiplier` _asthird_person_game_mode_2) 1)) _asthird_person_game_mode_2)
  (bind _asthird_person_character (cast `/Game/ThirdPersonBP/Blueprints/ThirdPersonCharacter` (`GameplayStatics.GetPlayerCharacter` 0)))
  (bind _charactermovement (`Character.CharacterMovement` _asthird_person_character))
  (set `CharacterMovementComponent.MaxWalkSpeed` (`KismetMathLibrary.FClamp` (* (`CharacterMovementComponent.MaxWalkSpeed` _charactermovement) 1.5) 600.0 1200.0) _charactermovement)
  (`KismetSystemLibrary.Delay` 0.5)
  (`self.K2_DestroyActor`))

(fn `SpawnObstacles`
  (switch `int` (`KismetMathLibrary.RandomIntegerInRange` 0 6)
    (:`1`
      (`|SpawnActorFromClass` "/Game/RunnerGame/Blueprints/Obstacle.Obstacle_C" (`SceneComponent.K2_GetComponentToWorld` (`self.Arrow_Lane_One`)) "AdjustIfPossibleButAlwaysSpawn" "OverrideRootScale" null null))
    (:`4`
      (`|SpawnActorFromClass` "/Game/RunnerGame/Blueprints/Obstacle.Obstacle_C" (`SceneComponent.K2_GetComponentToWorld` (`self.Arrow_Lane_Two`)) "AdjustIfPossibleButAlwaysSpawn" "OverrideRootScale" null null))
    (:`6`
      (`|SpawnActorFromClass` "/Game/RunnerGame/Blueprints/Obstacle.Obstacle_C" (`SceneComponent.K2_GetComponentToWorld` (`self.Arrow_Lane_Three`)) "AdjustIfPossibleButAlwaysSpawn" "OverrideRootScale" null null))))

(fn `UserConstructionScript`)